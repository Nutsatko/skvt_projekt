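; BP_WallSconce is a wall sconce light with configurable on/off state, brightness, color and cone angles.
; The construction script applies these variables to the SconceLight component, whose inner and outer cone settings shape its beam.
; ToggleON stores a new on/off state in IsON and updates the light's visibility to match.
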(fn `Toggle ON`
  (params (`Set On` :type Boolean))
  (bind _output_get (set `self.Is ON` `Set On`))
  (`SceneComponent.SetVisibility` (`self.SconceLight`) _output_get false))

(fn `UserConstructionScript`
  (bind _sconcelight (`self.SconceLight`))
  (`SceneComponent.SetVisibility` (`self.SconceLight`) (`self.Is ON`) false)
  (`LightComponent.SetIntensity` _sconcelight (`self.Brightness`))
  (`LightComponent.SetLightColor` _sconcelight (`self.Color`) true)
  (`SpotLightComponent.SetInnerConeAngle` _sconcelight (`self.Inner Cone Angle`))
  (`SpotLightComponent.SetOuterConeAngle` _sconcelight (`self.Outer Cone Angle`)))